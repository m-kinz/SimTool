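; Actor that slices a deformed Flex soft body and writes mesh data to files for each stage.
; After a deformation delay, it saves the skinned Flex vertices and converts them to a procedural mesh.
; It cuts this along Y at bounds-derived planes, respawning each piece as a Flex actor using the original soft settings.
; Initial slice geometry is stored at spawn, and deformed slice vertices and normals after another delay.
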(event EventBeginPlay
  (bind _returnvalue (Class|Actor|GetActorLabel))
  (bind (_origin _boxextent) (Collision|GetActorBounds false))
  (bind _flex (Variables|Default|GetFlex))
  (bind _totalnumbercuts (Variables|Default|GetTotalNumberCuts))
  (bind _cut_positions (Variables|Default|GetCut%20Positions))
  (bind _outputfolder (Variables|Default|GetOutputFolder))
  (bind _outputfolder_2 (Variables|Default|GetOutputFolder))
  (bind _returnvalue_2 (/ _totalnumbercuts 2))
  (bind _returnvalue_3 (Utilities|String|Append _outputfolder "\\Initial"))
  (bind _returnvalue_4 (Utilities|String|Append _outputfolder_2 "\\Slices deformed"))
  ;[1 1 1] Get Settings from Flex Component, shortcut this if you want to set the variables yourself
  (bind (_particlespacing _volumesampling _surfacesampling _clusterspacing _clusterradius _clusterstiffness _container) (Class|MyBlueprintFunctionLibrary|GetFlexSoftSettings (Variables|Default|GetFlex)))
  (Variables|Default|SetParticleSpacing _particlespacing)
  (Variables|Default|SetVolumeSampling _volumesampling)
  (Variables|Default|SetClusterSpacing _clusterspacing)
  (Variables|Default|SetSurfaceSampling _surfacesampling)
  (Variables|Default|SetClusterRadius _clusterradius)
  (Variables|Default|SetClusterStiffness _clusterstiffness)
  (Variables|Default|SetContainer _container)
  ;[1 1 1] Store initial object
  (bind (_vertices _triangles _normals _uvs) (Class|KismetProceduralMeshLibrary|GetSectionfromStaticMesh (Variables|/Script/Engine.StaticMeshComponent|GetStaticMesh (Variables|Default|GetFlex))))
  (Class|MyBlueprintFunctionLibrary|WriteVectorDataIntoFile _vertices _returnvalue_3 _returnvalue ".xyz")
  (Class|MyBlueprintFunctionLibrary|WriteTriangleDataIntoFile _triangles _returnvalue_3 _returnvalue ".triangle")
  (Utilities|FlowControl|Delay (Variables|Default|GetDeformation%20Delay))
  ;[1 1 1] Store deformed object and convert to Procedural Mesh Component
  (Development|PrintString "Convert")
  (bind (_vertices_2 _normals_2 _tangents _meanrotation _meantranslation) (Class|MyBlueprintFunctionLibrary|Skin _flex))
  (bind _transformedvertices (CallFunction|Transform _meanrotation _meantranslation _flex _vertices_2))
  (Class|MyBlueprintFunctionLibrary|WriteVectorDataIntoFile _transformedvertices (Utilities|String|Append (Variables|Default|GetOutputFolder) "\\Deformed") (Class|Actor|GetActorLabel) ".xyz")
  (Class|ProceduralMeshComponent|CreateMeshSectionLinearColor (Variables|Default|GetProceduralMesh) 0 _vertices_2 _triangles _normals_2 _uvs 0 _tangents false)
  (Components|DestroyComponent (Variables|Default|GetFlex))
  (Utilities|FlowControl|Delay 0.1)
  ;[1 1 1] Calculate cut positions
  (Variables|Default|SetPMC%20to%20spawn (Variables|Default|GetProceduralMesh))
  (bind _output_get (Variables|Default|SetNumberCutPlane _returnvalue_2))
  (bind _output_get_2 (Variables|Default|SetBoxExtendY (Math|Vector|MakeVector 0.0 (.Y (Math|Vector|BreakVector (/ _boxextent (/ (Math|Conversions|ToFloat(Integer) (+ _totalnumbercuts 1)) 1.3)))) 0.0)))
  (if (!= _totalnumbercuts 1) ; If only one slice
    (while (>= _output_get (* _returnvalue_2 -1))
      (if (!= _output_get 0) ; Skip cut in middle
        (Utilities|Array|AppendArray _cut_positions (Utilities|Array|MakeArray (+ _origin (* _output_get_2 _output_get)))))
      (Variables|Default|SetNumberCutPlane (- (Variables|Default|GetNumberCutPlane) 1)))
    (else
      (Utilities|Array|AppendArray _cut_positions (Utilities|Array|MakeArray (+ _origin (Math|Conversions|ToVector(Float) (* (.Y (Math|Vector|BreakVector _boxextent)) 0.8)))))))
  ;[1 1 1] Slice object
  (for _array_element _cut_positions
    (bind _outotherhalfprocmesh (Class|KismetProceduralMeshLibrary|SliceProceduralMesh (Variables|Default|GetPMC%20to%20spawn) _array_element "0.000000,1.000000,0.000000" true "UseLastSectionForCap"))
    (CallFunction|SpawnFlexActor (Variables|Default|GetPMC%20to%20spawn))
    (Variables|Default|SetPMC%20to%20spawn _outotherhalfprocmesh)
    (Utilities|FlowControl|Delay (Variables|Default|GetSpawnDelay)))
  (CallFunction|SpawnFlexActor (Variables|Default|GetPMC%20to%20spawn))
  (Utilities|FlowControl|Delay (Variables|Default|GetDeformation%20Delay))
  ;[1 1 1] Store deformed slices
  (Development|PrintString "Store slices")
  (for (_array_element_2 _array_index) (Variables|Default|GetFlexSlices)
    (bind (_vertices_3 _normals_3) (Class|MyBlueprintFunctionLibrary|Skin _array_element_2))
    (Class|MyBlueprintFunctionLibrary|WriteVectorDataIntoFile _vertices_3 _returnvalue_4 (Utilities|String|Append (Class|Actor|GetActorLabel) "_slice" (Utilities|String|ToString(Integer) _array_index)) ".xyz")
    (Class|MyBlueprintFunctionLibrary|WriteVectorDataIntoFile _normals_3 _returnvalue_4 (Utilities|String|Append (Class|Actor|GetActorLabel) "_slice" (Utilities|String|ToString(Integer) _array_index)) ".normals")))

(fn ConstructionScript)

(fn SpawnFlexActor
  (params (ProcMesh :type Procedural%20Mesh%20Component%20Object%20Reference))
  (bind _outputfolder (Variables|Default|GetOutputFolder))
  (bind _returnvalue (Utilities|String|Append _outputfolder "\\Slices"))
  ;[1 1 1] Convert Procedural Mesh Component to Flex Static Mesh and set in actor
  (bind _returnvalue_2 (Class|MyBlueprintFunctionLibrary|PMCtoFlex ProcMesh (Variables|Default|GetNumberSlice) (Variables|Default|GetParticleSpacing) (Variables|Default|GetVolumeSampling) (Variables|Default|GetSurfaceSampling) (Variables|Default|GetClusterSpacing) (Variables|Default|GetClusterRadius) (Variables|Default|GetClusterStiffness) (Variables|Default|GetContainer))) ; Convert Procedural Mesh Component to Flex Static Mesh
  ;[1 1 1] Spawn new Flex Actor for slice
  (bind _returnvalue_3 (Game|SpawnActorfromClass "/Script/Flex.FlexActor" (Math|Transform|ComposeTransforms (Transformation|GetWorldTransform ProcMesh) (Math|Transform|MakeTransform (Math|Vector|MakeVector 0.0 (Math|Conversions|ToFloat(Integer) (* (Variables|Default|GetNumberSlice) 300)) 1e+02))) "Undefined" 0 0))
  (Components|DestroyComponent ProcMesh) ; Destroy the Procedural Mesh Component Slice
  (bind _output_get (LocalVariables|SetNew%20Label (Utilities|String|Append (Utilities|String|Append (Class|Actor|GetActorLabel) "_slice") (Utilities|String|ToString(Integer) (Variables|Default|GetNumberSlice)))))
  (EditorScripting|ActorEditing|SetActorLabel _returnvalue_3 _output_get true)
  (Components|StaticMesh|SetStaticMesh (Variables|/Script/Engine.StaticMeshActor|GetStaticMeshComponent _returnvalue_3) _returnvalue_2) ; Set Flex Static Mesh for Actor
  (Class|MyBlueprintFunctionLibrary|ReregisterFlexComponent (Actor|GetComponentbyClass _returnvalue_3 "/Script/Flex.FlexComponent")) ; Reregister to enable simulation
  (Utilities|Array|Add (Variables|Default|GetFlexSlices) (Actor|GetComponentbyClass _returnvalue_3 "/Script/Flex.FlexComponent")) ; Add to array for storing deformed later
  ;[1 1 1] Store initial slices
  (bind (_vertices _triangles) (Class|KismetProceduralMeshLibrary|GetSectionfromStaticMesh _returnvalue_2))
  (Class|MyBlueprintFunctionLibrary|WriteTriangleDataIntoFile _triangles _returnvalue (LocalVariables|GetNew%20Label) ".triangle")
  (Class|MyBlueprintFunctionLibrary|WriteVectorDataIntoFile _vertices _returnvalue (LocalVariables|GetNew%20Label) ".xyz")
  (Variables|Default|SetNumberSlice (+ (Variables|Default|GetNumberSlice) 1)))

(fn Transform
  (params (NewParam :type Rotator) (NewParam1 :type Vector) (NewParam3 :type Flex%20Component%20Object%20Reference) (NewParam2 :type Array%20of%20Vectors))
  (bind _transformedvectors (LocalVariables|GetTransformedVectors))
  (for _array_element NewParam2
    (Utilities|Array|AppendArray _transformedvectors (Utilities|Array|MakeArray (Math|Vector|RotateVector (+ _array_element NewParam1) (Class|KismetMathLibrary|NegateRotator NewParam)))))
  (return _transformedvectors))